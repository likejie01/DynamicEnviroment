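; Construction-time tool actor that places rows of lights along a spline, as either point lights or emissive material billboards.
; It spaces them evenly by distance, offsetting rows on local Y, then applies intensity and optional random color.
; Billboards share one dynamic material, which also carries the flash parameter.
; ReSetLightIntensity rescales brightness and visibility afterward; the camera-distance attenuation logic is unconnected.
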(event `self.ReceiveTick`
  (params (DeltaSeconds :type "Float (single-precision)")))

(event `ReSetLightIntensity`
  (params (Visible :type Boolean) (IntensityScale :type "Float (double-precision)"))
  (bind _returnvalue (* IntensityScale (`self.LightIntensity`)))
  (bind _returnvalue_2 (* IntensityScale (`self.Intensity`)))
  (if (`self.UseLight`)
    (for _array_element (`self.PointLightComponents`)
      (`LightComponent.SetIntensity` _array_element _returnvalue)
      (`SceneComponent.SetVisibility` _array_element (and Visible (!= _returnvalue 0.0)) false))
    (else
      (`MaterialInstanceDynamic.SetScalarParameterValue` (`self.DynamicMaterial`) "EmissiveIntensity" _returnvalue_2)
      (for _array_element_2 (`self.BillboardComponent`)
        (`SceneComponent.SetVisibility` _array_element_2 (and Visible (!= _returnvalue_2 0.0)) false)))))

(event `SetSpline`
  (`SplineComponent.SetClosedLoop` (`self.Spline`) (`self.SplineIsClosed`) true))

(event `SpawnLight`
  (bind _spline (`self.Spline`))
  (bind _numofrow (`self.NumOfRow`))
  (bind _offsetinterval (`self.OffsetInterval`))
  (bind _offsetinterval_2 (`self.OffsetInterval`))
  (bind _screensize (`self.ScreenSize`))
  (bind _sizeinscreen (`self.SizeInScreen`))
  (bind _transformcache (`self.TransformCache`))
  (bind _returnvalue (- (`self.NumOfLight`) 1))
  (bind _returnvalue_2 (select `bool` _sizeinscreen :`false` (* _screensize 16000.0) :`true` _screensize))
  (`KismetArrayLibrary.Array_Clear` (`self.PointLightComponents`))
  (`KismetArrayLibrary.Array_Clear` (`self.BillboardComponent`))
  (bind _returnvalue_3 (`KismetMaterialLibrary.CreateDynamicMaterialInstance` (`self.Material`)))
  (`self.Set Dynamic Material` _returnvalue_3)
  (for _index (range (+ _returnvalue 1))
    (for _index_2 (range _numofrow)
      (if (== (mod _numofrow 2) 1)
        (if (== (mod _index_2 2) 1)
          (bind _returnvalue_4 (`KismetMathLibrary.Conv_IntToDouble` (* _index (/ (`SplineComponent.GetSplineLength` (`self.Spline`)) _returnvalue))))
          (bind (_x _y _z) (`KismetMathLibrary.BreakVector3f` (`SplineComponent.GetLocationAtDistanceAlongSpline` _spline _returnvalue_4 "Local")))
          (bind _returnvalue_5 (`SplineComponent.GetRotationAtDistanceAlongSpline` _spline _returnvalue_4 "Local"))
          (set `self.TransformCache` (`KismetMathLibrary.MakeTransform` (`KismetMathLibrary.MakeVector` _x (+ (* (/ (+ _index_2 1) 2) _offsetinterval_2) _y) _z) _returnvalue_5))
          (else
            (set `self.TransformCache` (`KismetMathLibrary.MakeTransform` (`KismetMathLibrary.MakeVector` _x (- _y (* _offsetinterval_2 (/ _index_2 2))) _z) _returnvalue_5))))
        (elif (== (mod _index_2 2) 1)
          (set `self.TransformCache` (`KismetMathLibrary.MakeTransform` (`KismetMathLibrary.MakeVector` _x (- _y (* (/ _index_2 2) _offsetinterval)) _z) _returnvalue_5))
          (else
            (set `self.TransformCache` (`KismetMathLibrary.MakeTransform` (`KismetMathLibrary.MakeVector` _x (+ _y (* _offsetinterval (/ (+ _index_2 1) 2))) _z) _returnvalue_5)))))
      (if (`self.UseLight`)
        (bind _returnvalue_6 (`|AddComponentByClass` "/Script/Engine.PointLightComponent" false _transformcache))
        (`KismetArrayLibrary.Array_Add` (`self.PointLightComponents`) _returnvalue_6)
        (else
          (bind _returnvalue_7 (`AddComponent|NODE_AddMaterialBillboardComponent-0` :`RelativeTransform` _transformcache))
          (`MaterialBillboardComponent.AddElement` _returnvalue_7 (`self.DynamicMaterial`) null _sizeinscreen _returnvalue_2 _returnvalue_2 (`self.DistanceToSize`))
          (`KismetArrayLibrary.Array_Add` (`self.BillboardComponent`) _returnvalue_7))))))

(event `SetPointLightComponents`
  (bind _randomcolor (`self.RandomColor`))
  (bind _randominterval (`self.RandomInterval`))
  (bind _dynamicmaterial (`self.DynamicMaterial`))
  (bind _color (`self.Color`))
  (bind _lightcolor (`self.LightColor`))
  (bind (_r _g _b _a) (`KismetMathLibrary.BreakColor` _lightcolor))
  (bind _returnvalue (`KismetMathLibrary.RandomFloatInRange` 0.0 _randominterval))
  (bind _returnvalue_2 (`KismetMathLibrary.RandomFloatInRange` 0.0 _randominterval))
  (bind (_r_2 _g_2 _b_2 _a_2) (`KismetMathLibrary.BreakColor` _color))
  (if (`self.UseLight`)
    (for _array_element (`self.PointLightComponents`)
      (`LocalLightComponent.SetIntensityUnits` _array_element "Lumens")
      (`LightComponent.SetIntensity` _array_element (`self.LightIntensity`))
      (`LocalLightComponent.SetAttenuationRadius` _array_element (`self.LightRadius`))
      (`LightComponent.SetLightColor` _array_element (`KismetMathLibrary.SelectColor` (`KismetMathLibrary.MakeColor` (+ _r _returnvalue) (+ _g _returnvalue_2) (+ _b (`KismetMathLibrary.RandomFloatInRange` 0.0 _randominterval)) _a) _lightcolor _randomcolor) true)
      (`LightComponentBase.SetCastShadows` _array_element (`self.CastShadow`)))
    (else
      (`MaterialInstanceDynamic.SetScalarParameterValue` _dynamicmaterial "EmissiveIntensity" (`self.Intensity`))
      (`MaterialInstanceDynamic.SetVectorParameterValue` _dynamicmaterial "EmissiveColor" (`KismetMathLibrary.SelectColor` (`KismetMathLibrary.MakeColor` (+ _returnvalue _r_2) (+ _returnvalue_2 _g_2) (+ 0.0 _b_2) _a_2) _color _randomcolor))
      (`MaterialInstanceDynamic.SetScalarParameterValue` _dynamicmaterial "Flash" (`KismetMathLibrary.Conv_BoolToDouble` (`self.IsFlash`))))))

(fn `Set Dynamic Material`
  (params (In :type "MaterialInstanceDynamic Object Reference"))
  (`MaterialInstanceDynamic.SetScalarParameterValue` In "EmissiveIntensity" (`self.Intensity`))
  (`MaterialInstanceDynamic.SetVectorParameterValue` In "EmissiveColor" (`self.Color`))
  (set `self.DynamicMaterial` In))

(fn `UserConstructionScript`
  (`|ExecutionSequence`
    (:`then_0`
      (`self.SetSpline`))
    (:`then_1`
      (`self.SpawnLight`))
    (:`then_2`
      (`self.SetPointLightComponents` :!label _label))
    (:`then_3`
      (if (`self.RandomColor`)
        (goto _label)))
    (:`then_4`
      (if (`self.IsFlash`)
        (goto _label)))))